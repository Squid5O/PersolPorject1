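; Player character Blueprint, apparently the protagonist, that handles basic forward and sideways movement input.
; MoveForward and MoveRight axis events add movement along the forward and right vectors of the control rotation, scaled by axis value.
; Both use the full control rotation rather than yaw alone, and are skipped while the DisableMovement flag is set.
; The construction script and other events are empty.
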(event EventBeginPlay)

(event Collision|EventActorBeginOverlap
  (params (OtherActor :type Actor%20Object%20Reference)))

(event EventTick
  (params (DeltaSeconds :type Float%20%28single-precision%29)))

(event Input|ActionEvents|InputActionWWW
  (params (Key :type Key%20Structure :default "None")))

(event Input|ActionEvents|InputActionAAA
  (params (Key :type Key%20Structure :default "None")))

(event Input|ActionEvents|InputActionSSS
  (params (Key :type Key%20Structure :default "None")))

(event Input|ActionEvents|InputActionDDD
  (params (Key :type Key%20Structure :default "None")))

(event Input|AxisEvents|InputAxisMoveForward
  (params (AxisValue :type Float%20%28single-precision%29))
  (bind _returnvalue (Pawn|GetControlRotation :!class /Script/Engine.Pawn))
  (bind (_roll _pitch _yaw) (Math|Rotator|BreakRotator _returnvalue))
  (if (not (Variables|Default|GetDisableMovement))
    (Pawn|Input|AddMovementInput (Math|Vector|GetForwardVector (Math|Rotator|MakeRotator _roll _pitch _yaw)) AxisValue false)))

(event Input|AxisEvents|InputAxisMoveRight
  (params (AxisValue :type Float%20%28single-precision%29))
  (bind _returnvalue (Pawn|GetControlRotation :!class /Script/Engine.Pawn))
  (bind (_roll _pitch _yaw) (Math|Rotator|BreakRotator _returnvalue))
  (if (not (Variables|Default|GetDisableMovement))
    (Pawn|Input|AddMovementInput (Math|Vector|GetRightVector (Math|Rotator|MakeRotator _roll _pitch _yaw)) AxisValue false)))

(fn ConstructionScript)